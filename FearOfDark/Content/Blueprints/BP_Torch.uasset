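; BP_Torch is a torch that can be grabbed with a motion controller and switched on and off.
; Grab stores the controller and attaches the torch to it, keeping its world transform.
; Release detaches the torch only if the releasing controller matches the stored one, so releasing another object does not drop it.
; Interact toggles the visibility of the TorchLight component.
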(event EventInteract
  (bind _torchlight (Variables|Default|GetTorchLight))
  ;[1 1 1] Turns Torch on and off
  (if (Rendering|IsVisible _torchlight)
    (Rendering|SetVisibility _torchlight false false)
    (else
      (Rendering|SetVisibility _torchlight true false))))

(event EventGrab
  (params (Motion%20Controller :type Motion%20Controller%20Component%20Object%20Reference))
  (bind _output_get (Variables|Default|SetMotion%20Controller Motion%20Controller))
  (Transformation|AttachComponentToComponent _output_get "" "KeepWorld" "KeepWorld" "KeepWorld" true))

(event EventRelease
  (params (Motion%20Controller :type Motion%20Controller%20Component%20Object%20Reference))
  ;[1 1 1] Makes sure when releasing another object it doesnt release the torch
  (if (== Motion%20Controller (Variables|Default|GetMotion%20Controller))
    (Transformation|DetachFromActor "KeepWorld" "KeepWorld" "KeepWorld")))

(fn ConstructionScript)