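; BP_Door is a hinged door that a motion controller can swing by its handle once its keyhole is unlocked.
; Grab stores the controller as the hand if it is within the handle's collision sphere, and Release clears it.
; Tick locks the door while shut with the keyhole locked, otherwise plays a one-time unlock sound.
; When unlocked, yaw tracks the held hand within clamped limits, and a released door snaps shut when nearly closed.
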(event EventGrab
  (params (Motion%20Controller :type Motion%20Controller%20Component%20Object%20Reference))
  (bind _handle_collision (Variables|Default|GetHandle%20Collision))
  (if (Utilities|Operators|EqualEqual (Transformation|GetWorldLocation Motion%20Controller) (Transformation|GetWorldLocation _handle_collision) (Variables|/Script/Engine.SphereComponent|GetSphereRadius _handle_collision))
    (Variables|Default|SetHand Motion%20Controller)
    (Development|PrintString "Grabbed")))

(event EventRelease
  (params (Motion%20Controller :type Motion%20Controller%20Component%20Object%20Reference))
  (if (== Motion%20Controller (Variables|Default|GetHand))
    (Variables|Default|SetHand 0)))

(event EventTick
  (params (DeltaSeconds :type Float%20%28single-precision%29))
  (bind _hand (Variables|Default|GetHand))
  (bind _door (Variables|Default|GetDoor))
  ;[1 1 1] Is the door unlocked
  (Utilities|FlowControl|Sequence
    (:then_0
      (if (and (not (Variables|/Game/Blueprints/BP_KeyHole.BP_KeyHole_C|GetUnlocked (Variables|Default|GetKey%20Hole))) (Math|Float|NearlyEqual(Float) (.yaw (Transformation|GetWorldRotation (Variables|Default|GetDoor))) 0.0 1e-06))
        (Variables|Default|SetLocked true)
        (else
          (Variables|Default|SetLocked false)
          (Utilities|FlowControl|DoOnce false
            (:Completed
              (Audio|PlaySoundatLocation "/Game/door-unlock-92281.door-unlock-92281" "0, 0, 0" "0, 0, 0" 1.0 1.0 0.0 0 0 0 0))))))
    (:then_1
      (if (not (Variables|Default|GetLocked))
        (Utilities|IsValid _hand
          (:Is%20Valid
            (Transformation|SetWorldRotation _door (Math|Rotator|MakeRotator 0.0 0.0 (Math|Float|ClampAngle (- (.yaw (Math|Rotator|FindLookatRotation (Transformation|GetWorldLocation _hand) (Transformation|GetWorldLocation _door))) 9e+01) -9e+01 9e+01)) false false))
          (:Is%20Not%20Valid
            (if (Math|Float|NearlyEqual(Float) (.yaw (Transformation|GetWorldRotation _door)) 0.0 1e+01)
              (Transformation|SetWorldRotation _door "0, 0, 0" false false))))))))

(fn ConstructionScript)