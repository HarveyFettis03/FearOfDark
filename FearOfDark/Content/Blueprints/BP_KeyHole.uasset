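; VR keyhole actor that captures a bp_Key near its entry point and tracks an Unlocked state.
; Tick sphere-checks the spline's entry, detaches a detected key, then slides it along the start-to-end segment by projecting the motion controller's position.
; Reaching the entry reattaches the key to the controller and sets Unlocked.
; Without a controller, a key near the end attaches and unlocks; otherwise it is dropped with physics.
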(event EventBeginPlay
  (bind _spline (Variables|Default|GetSpline))
  (Variables|Default|SetStartPoint (Spline|GetLocationatSplinePoint _spline 1 "World"))
  (Variables|Default|SetEndPoint (Spline|GetLocationatSplinePoint _spline 0 "World")))

(event EventTick
  (params (DeltaSeconds :type Float%20%28single-precision%29))
  (Utilities|IsValid (Variables|Default|GetKey)
    (:Is%20Valid
      ;[1 1 1] Key unlocking door
      (Utilities|IsValid (Variables|/Game/Blueprints/bp_Key.bp_Key_C|GetMotion%20Controller (Variables|Default|GetKey))
        (:Is%20Valid
          (Transformation|SetActorLocation (Variables|Default|GetKey) (Math|Vector|FindClosestPointonSegment (Transformation|GetWorldLocation (Variables|/Game/Blueprints/bp_Key.bp_Key_C|GetMotion%20Controller (Variables|Default|GetKey))) (Variables|Default|GetStartPoint) (Variables|Default|GetEndPoint)) false false)
          (if (Utilities|Operators|EqualEqual (Transformation|GetActorLocation (Variables|Default|GetKey)) (Variables|Default|GetStartPoint) 1e+01)
            (Transformation|AttachComponentToComponent (Variables|Default|GetKey) (Variables|/Game/Blueprints/bp_Key.bp_Key_C|GetMotion%20Controller (Variables|Default|GetKey)) "None" "KeepRelative" "KeepRelative" "KeepRelative" true)
            (Variables|Default|SetKey 0)
            (Variables|Default|SetUnlocked true)))
        (:Is%20Not%20Valid
          ;[1 1 1] Attach Key
          (if (Utilities|Operators|EqualEqual (Transformation|GetActorLocation (Variables|Default|GetKey)) (Variables|Default|GetEndPoint) 3e+01)
            (Variables|Default|SetUnlocked true)
            (Transformation|SetActorLocation (Variables|Default|GetKey) (Variables|Default|GetEndPoint) false false)
            (Transformation|AttachActorToActor (Variables|Default|GetKey) self "None" "KeepWorld" "KeepWorld" "KeepWorld" true)
            (Physics|SetSimulatePhysics (Variables|/Game/Blueprints/bp_Key.bp_Key_C|GetKey%20Mesh (Variables|Default|GetKey)) true)
            (else
              (Physics|SetSimulatePhysics (Variables|/Game/Blueprints/bp_Key.bp_Key_C|GetKey%20Mesh (Variables|Default|GetKey)) true)
              (Variables|Default|SetKey 0))))))
    (:Is%20Not%20Valid
      ;[1 1 1] Detect Key
      (bind _outactors (Collision|SphereOverlapActors (Variables|Default|GetStartPoint) 2e+01 (Utilities|Array|MakeArray "ObjectTypeQuery2") 0))
      (bind _array_element (Utilities|Array|ForEachLoopwithBreak _outactors :!label _label)
        (:LoopBody
          (bind _asbp_key (Utilities|Casting|CastTobp_Key _array_element))
          (bind _output_get (Variables|Default|SetKey _asbp_key))
          (Transformation|DetachFromActor _output_get "KeepWorld" "KeepWorld" "KeepWorld")
          (goto _label Break))))))

(fn ConstructionScript)